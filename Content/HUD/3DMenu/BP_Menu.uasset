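; BP_Menu is a 3D menu actor that hosts a widget and moves the player's view to other linked menu actors.
; On BeginPlay it binds to the transition event of its WBP_MenuBaseClass widget and disables its own collision.
; The widget passes an index into LinkedMenus, and a valid one triggers an eased view-target blend to that menu.
; Each transition switches collision off on the current menu and on for the destination.
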(event `self.ReceiveBeginPlay`
  (bind _aswbp_main_menu_base_class (cast `/Game/HUD/3DMenu/WBP_MenuBaseClass` (`WidgetComponent.GetUserWidgetObject` (`self.Widget`))))
  (add `/Game/HUD/3DMenu/WBP_MenuBaseClass.TransitionToLinkedMenu` _aswbp_main_menu_base_class (delegate `OnTransitionBetweenMenus`))
  (`self.SetActorEnableCollision` false))

(event `OnTransitionBetweenMenus`
  (params (MenuIndex :type Integer))
  (if (`KismetArrayLibrary.Array_IsValidIndex` (`self.LinkedMenus`) MenuIndex)
    (`self.Transition To` (`|GetArrayItem` (`self.LinkedMenus`) MenuIndex))))

(event `Transition To`
  (params (NewMenu :type "/Game/HUD/3DMenu/BP_Menu Object Reference"))
  (`self.SetActorEnableCollision` false)
  (`self.SetActorEnableCollision` NewMenu true)
  (`PlayerController.SetViewTargetWithBlend` (`GameplayStatics.GetPlayerController` 0) NewMenu 2.0 "VTBlend_EaseInOut" 2.0 false))

(fn `UserConstructionScript`)