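; Pushable object that the player character (Zazi) can push with the Harness ability.
; Collider overlap sets or clears the character's CurrentPush, registering only when that ability is equipped.
; Interact finds the nearest in-range PushTransform, checks standing room, walkable floor and obstructions with traces, then teleports the character there and triggers the ability.
; The construction script shows each push transform as an arrow, and failed checks print on-screen errors.
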(event `self.PickUpCollider.OnComponentBeginOverlap`
  (params (OverlappedComponent :type "PrimitiveComponent Object Reference") (OtherActor :type "Actor Object Reference") (OtherComp :type "PrimitiveComponent Object Reference") (OtherBodyIndex :type Integer) (bFromSweep :type Boolean) (SweepResult :type "HitResult Structure (by ref)"))
  ;[1 1 1] Initialize Zazi's current pushable object
  (bind _asbp_player_controller (cast `/Game/Blueprints/PlayerController/BP_PlayerController` OtherActor))
  (bind _output_get (set `self.Character` _asbp_player_controller))
  (bind _current_ability (`/Game/Blueprints/PlayerController/BP_PlayerController.Current Ability` _output_get)
    (:`then`
      (if (== (`Ability.AbilityID` _current_ability) 4)
        (set `/Game/Blueprints/PlayerController/BP_PlayerController.Current Push` self (`self.Character`))))
    (:`else`
      (`self.Err Log` "Harness Ability is not equipped"))))

(event `self.PickUpCollider.OnComponentEndOverlap`
  (params (OverlappedComponent :type "PrimitiveComponent Object Reference") (OtherActor :type "Actor Object Reference") (OtherComp :type "PrimitiveComponent Object Reference") (OtherBodyIndex :type Integer))
  ;[1 1 1] Remove Zazi's current pushable object
  (bind _asbp_player_controller (cast `/Game/Blueprints/PlayerController/BP_PlayerController` OtherActor))
  (`/Engine/EditorBlueprintResources/StandardMacros.IsValid` (`/Game/Blueprints/PlayerController/BP_PlayerController.Current Push` _asbp_player_controller)
    (:`Is Valid`
      (set `/Game/Blueprints/PlayerController/BP_PlayerController.Current Push` null _asbp_player_controller))
    (:`Is Not Valid`
      (`self.Err Log` "No valid push object"))))

(event `self.Interact`
  (bind _characternewtransform_location (`KismetMathLibrary.BreakTransform` (`self.CharacterNewTransform`)))
  (bind _characternewtransform_location_2 (`KismetMathLibrary.BreakTransform` (`self.CharacterNewTransform`)))
  (bind _capsulecomponent (`Character.CapsuleComponent` (`self.Character`)))
  ;[1 1 1] All the logic for getting the push location
  (bind _closest_transform (`self.Find Closest Push Transform Index` (`KismetMathLibrary.Conv_VectorToVector2D` (`self.K2_GetActorLocation` (`self.Character`))) (`self.Push Range`)))
  (if (>= _closest_transform 0)
    (bind (_returnvalue_location _returnvalue_rotation) (`KismetMathLibrary.BreakTransform` (`KismetMathLibrary.ComposeTransforms` (`|GetArrayItem` (`self.Push Transforms`) _closest_transform) (`self.GetTransform`))))
    (bind _output_get (set `self.CharacterNewTransform` (`KismetMathLibrary.MakeTransform` (+ _returnvalue_location (`KismetMathLibrary.MakeVector` 0.0 0.0 (`CapsuleComponent.GetScaledCapsuleHalfHeight` (`Character.CapsuleComponent` (`self.Character`))))) _returnvalue_rotation))) ; Keep track of which transform I gotta move to
    (`KismetSystemLibrary.DrawDebugSphere` (.location _output_get) 20.0 12 (struct :`R` 1.0 :`G` 1.0 :`B` 1.0 :`A` 1.0) 2.0 1.0)
    (bind _outhit (`KismetSystemLibrary.CapsuleTraceSingle` :`Start` (+ _characternewtransform_location (0.0 0.0 300.0)) :`End` (- _characternewtransform_location (0.0 0.0 100.0)) :`Radius` (`CapsuleComponent.GetScaledCapsuleRadius` _capsulecomponent) :`HalfHeight` (`CapsuleComponent.GetScaledCapsuleHalfHeight` _capsulecomponent) :`TraceChannel` "TraceTypeQuery1" :`DrawDebugType` "ForDuration")) ; Check if you're on a floor before we teleport to the location to start pushing
    (bind (_bblockinghit _binitialoverlap _time _distance _location _impactpoint _normal _impactnormal) (`GameplayStatics.BreakHitResult` _outhit))
    (if (not _binitialoverlap)
      (if (< (`CharacterMovementComponent.K2_GetWalkableFloorZ` (`Character.CharacterMovement` (`self.Character`))) (.z _impactnormal))
        (bind (_outhit_2 _returnvalue) (`KismetSystemLibrary.LineTraceSingle` (`self.K2_GetActorLocation`) _characternewtransform_location_2 "TraceTypeQuery1" false (`|MakeArray` (`self.Character`) (`/Game/Blueprints/PlayerController/BP_PlayerController.Current Ability` (`self.Character`)) :!type "Actor Object Reference") "ForDuration" true (struct :`B` 1.0 :`A` 1.0) (struct :`R` 1.0 :`B` 0.537673 :`A` 1.0))) ; Make sure there's nothing infront of the box
        (if (not _returnvalue)
          (`self.K2_SetActorTransform` (`self.Character`) (`self.CharacterNewTransform`) false true) ; Teleport to the push location
          (`Ability.AbilityPressed` (`/Game/Blueprints/PlayerController/BP_PlayerController.Current Ability` (`self.Character`))) ; Start the push logic
          (else
            (`self.Err Log` "Wall in between character and pushable")))
        (else
          (`self.Err Log` "Floor Not Walkable")))
      (else
        (`self.Err Log` "No Room To Stand")))
    (else
      (`self.Err Log` "No Push Transform Found"))))

(fn `Find Closest Push Transform Index`
  (params (`Character Loc` :type "Vector2D Structure") (`Push Range` :type "Float (double-precision)"))
  (returns (`Closest Transform` :type Integer))
  (locals (`Current Transform Index` :type Integer) (ClosestTransformIndex :type Integer :default -1) (`Current Distance Sq` :type "Float (double-precision)" :default 0.0) (ClosestDistanceSq :type "Float (double-precision)"))
  (for (_array_element _array_index) (`self.Push Transforms`)
    (set `local.Current Transform Index` _array_index)
    (bind _output_get (set `local.Current Distance Sq` (`KismetMathLibrary.DistanceSquared2D` (`KismetMathLibrary.Conv_VectorToVector2D` (`KismetMathLibrary.TransformLocation` (`self.GetTransform`) (.location _array_element))) (`local.Character Loc`))))
    (if (< _output_get (`KismetMathLibrary.Square` (`local.Push Range`)))
      (if (or (< (`local.ClosestTransformIndex`) 0) (< (`local.Current Distance Sq`) (`local.ClosestDistanceSq`)))
        (set `local.ClosestTransformIndex` (`local.Current Transform Index`))
        (set `local.ClosestDistanceSq` (`local.Current Distance Sq`)))))
  (return (`local.ClosestTransformIndex`)))

(fn `UserConstructionScript`
  (for _array_element (`self.Push Transforms`)
    (`AddComponent|NODE_AddArrowComponent-0` :`RelativeTransform` _array_element)))