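; Battery pickup that drives HUD and transition feedback when the player leaves its pickup collider.
; On end overlap it casts the game mode and the overlapping actor (as BP_PlayerController), then switches on that actor's BatteryCount.
; Counts one to five play the matching AddBattery animation on the game mode's HUD, and every count calls PlayBatteryTransition on the player.
; This graph only reads the count and never changes it.
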(event `self.PickUpCollider.OnComponentEndOverlap`
  (params (OverlappedComponent :type "PrimitiveComponent Object Reference") (OtherActor :type "Actor Object Reference") (OtherComp :type "PrimitiveComponent Object Reference") (OtherBodyIndex :type Integer))
  (bind _asbp_astro_shipping_co_game_mode (cast `/Game/Blueprints/GameMode/BP_AstroShippingCo_GameMode` (`GameplayStatics.GetGameMode`)))
  (bind _asbp_player_controller (cast `/Game/Blueprints/PlayerController/BP_PlayerController` OtherActor))
  (switch `int` (`AstroShippingCoCharacter.BatteryCount` _asbp_player_controller)
    (:`Default`
      (`AstroShippingCoCharacter.PlayBatteryTransition` _asbp_player_controller))
    (:`1`
      (bind _hud (`/Game/Blueprints/GameMode/BP_AstroShippingCo_GameMode.HUD` _asbp_astro_shipping_co_game_mode))
      (`UserWidget.PlayAnimation` _hud (`/Game/HUD/WBP_HUD.AddBattery1` _hud) 0.0 1 "Forward" 1.0 false)
      (`AstroShippingCoCharacter.PlayBatteryTransition` _asbp_player_controller))
    (:`2`
      (`UserWidget.PlayAnimation` _hud (`/Game/HUD/WBP_HUD.AddBattery2` _hud) 0.0 1 "Forward" 1.0 false)
      (`AstroShippingCoCharacter.PlayBatteryTransition` _asbp_player_controller))
    (:`3`
      (`UserWidget.PlayAnimation` _hud (`/Game/HUD/WBP_HUD.AddBattery3` _hud) 0.0 1 "Forward" 1.0 false)
      (`AstroShippingCoCharacter.PlayBatteryTransition` _asbp_player_controller))
    (:`4`
      (`UserWidget.PlayAnimation` _hud (`/Game/HUD/WBP_HUD.AddBattery4` _hud) 0.0 1 "Forward" 1.0 false)
      (`AstroShippingCoCharacter.PlayBatteryTransition` _asbp_player_controller))
    (:`5`
      (`UserWidget.PlayAnimation` _hud (`/Game/HUD/WBP_HUD.AddBattery5` _hud) 0.0 1 "Forward" 1.0 false)
      (`AstroShippingCoCharacter.PlayBatteryTransition` _asbp_player_controller))))

(fn `UserConstructionScript`)