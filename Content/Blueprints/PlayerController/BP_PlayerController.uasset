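; Player character Blueprint for Zazi, despite its controller name, handling ability input, health, menus and win/lose flow.
; Fire dispatches to CurrentAbility by AbilityID (heat gun, hover, dash, push), while FlipFlops toggle pause and inventory widgets.
; Tick opens the win map at the battery target; fatal damage opens game over.
; Hit and battery-pickup events swap eye expressions via dynamic materials, using montage notifies to time input locks and timeline-blended camera transitions.
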(event `InputAction|Fire`
  (params (Key :type "Key Structure"))
  ;[1 1 1] Harness
  (:`Pressed`
    (bind _current_ability (`self.Current Ability`)
      (:`then`
        (if (== (`Ability.AbilityID` _current_ability) 4)
          (bind _current_push (`self.Current Push`)
            (:`then`
              (`Interactable.Interact` _current_push))
            (:`else`))))
      (:`else`)))
  (:`Released`
    (bind _current_ability_2 (`self.Current Ability`)
      (:`then`
        (`Ability.AbilityReleased` _current_ability_2))
      (:`else`))))

(event `InputAction|Fire`
  (params (Key :type "Key Structure"))
  ;[1 1 1] Dash
  (:`Pressed`
    (bind _current_ability (`self.Current Ability`)
      (:`then`
        (if (== (`Ability.AbilityID` _current_ability) 3)
          (bind _asbp_ability_dash (cast `/Game/Blueprints/Abilities/BP_Ability_Dash` (`self.Current Ability`)))
          (`Ability.AbilityPressed` _asbp_ability_dash)))
      (:`else`)))
  (:`Released`
    (bind _asbp_ability_dash_2 (cast `/Game/Blueprints/Abilities/BP_Ability_Dash` (`self.Current Ability`)))
    (`Ability.AbilityReleased` _asbp_ability_dash_2)))

(event `InputAction|Fire`
  (params (Key :type "Key Structure"))
  ;[1 1 1] Hover
  (:`Pressed`
    (bind _current_ability (`self.Current Ability`)
      (:`then`
        (if (== (`Ability.AbilityID` _current_ability) 2)
          (bind _asbp_ability_hover (cast `/Game/Blueprints/Abilities/BP_Ability_Hover` (`self.Current Ability`)))
          (`Ability.AbilityPressed` _asbp_ability_hover)))
      (:`else`)))
  (:`Released`
    (bind _asbp_ability_hover_2 (cast `/Game/Blueprints/Abilities/BP_Ability_Hover` (`self.Current Ability`)))
    (`Ability.AbilityReleased` _asbp_ability_hover_2)))

(event `InputAxis|Hover`
  (params (AxisValue :type "Float (single-precision)"))
  (bind (_returnvalue_roll _returnvalue_pitch _returnvalue_yaw) (`KismetMathLibrary.BreakRotator` (`self.GetControlRotation`)))
  ;[1 1 1] Hover
  ;;[1 1 1] Launch Character Upwards
  (`self.AddMovementInput` (`KismetMathLibrary.GetUpVector` (`KismetMathLibrary.MakeRotator` 0.0 0.0 _returnvalue_yaw)) AxisValue))

(event `InputAction|Fire`
  (params (Key :type "Key Structure"))
  (bind _current_ability (`self.Current Ability`))
  ;[1 1 1] Heat Gun
  (:`Pressed`
    (`/Engine/EditorBlueprintResources/StandardMacros.IsValid` _current_ability
      (:`Is Valid`
        (if (== (`Ability.AbilityID` _current_ability) 1)
          (bind _asbp_ability_heat_gun (cast `/Game/Blueprints/Abilities/BP_Ability_HeatGun` (`self.Current Ability`)))
          (`Ability.AbilityPressed` _asbp_ability_heat_gun))))))

(event `InputAction|Pause Game` :paused true
  (params (Key :type "Key Structure"))
  ;[1 1 1] Pause Game
  (:`Pressed`
    (`/Engine/EditorBlueprintResources/StandardMacros.FlipFlop`
      (:`A`
        (bind _returnvalue (`|CreateWidget` "/Game/HUD/WBP_PauseMenu.WBP_PauseMenu_C"))
        (`UserWidget.AddToViewport` _returnvalue 0)
        (`GameplayStatics.SetGamePaused` true)
        (set `PlayerController.bShowMouseCursor` true (`GameplayStatics.GetPlayerController` 0)))
      (:`B`
        (`Widget.RemoveFromParent` _returnvalue)
        (`GameplayStatics.SetGamePaused` false)
        (set `PlayerController.bShowMouseCursor` false (`GameplayStatics.GetPlayerController` 0))))))

(event `InputAction|ShowInventory` :paused true
  (params (Key :type "Key Structure"))
  ;[1 1 1] Toggle Inventory
  (:`Pressed`
    (`/Engine/EditorBlueprintResources/StandardMacros.FlipFlop`
      (:`A`
        (bind _returnvalue (`|CreateWidget` "/Game/HUD/WBP_Inventory.WBP_Inventory_C"))
        (`UserWidget.AddToViewport` _returnvalue 0)
        (`GameplayStatics.SetGamePaused` true)
        (set `PlayerController.bShowMouseCursor` true (`GameplayStatics.GetPlayerController` 0)))
      (:`B`
        (if (`Widget.IsInViewport` _returnvalue)
          (`Widget.RemoveFromParent` _returnvalue)
          (`GameplayStatics.SetGamePaused` false)
          (set `PlayerController.bShowMouseCursor` false (`GameplayStatics.GetPlayerController` 0)))))))

(event `self.ReceiveTick`
  (params (DeltaSeconds :type "Float (single-precision)"))
  ;[1 1 1] Game Over after 2 Batteries Or health == 0
  (if (>= (`self.BatteryCount`) 5)
    (`KismetSystemLibrary.Delay` 3.0)
    (`GameplayStatics.OpenLevel` "GameWinMap")))

(event `Zazi Death`
  ;[1 1 1] Zazi Death Lose Condition
  (if (<= (`AC_HealthComponent.currentHealth` (`self.HealthComponent`)) 0.0)
    (`KismetSystemLibrary.Delay` 1.5)
    (`GameplayStatics.SetGamePaused` true)
    (`GameplayStatics.OpenLevel` "GameOverMap")))

(event `/Game/Blueprints/PlayerController/BPI_Damageable.Take Damage`
  (params (Damage :type "Float (single-precision)"))
  (bind _healthcomponent (`self.HealthComponent`))
  (bind _returnvalue (- (`AC_HealthComponent.currentHealth` _healthcomponent) Damage))
  ;[1 1 1] Player Takes Damage From Enemy
  (set `self.IsHit` true)
  (if (> _returnvalue 0.0)
    (set `AC_HealthComponent.currentHealth` _returnvalue _healthcomponent)
    (else
      (set `AC_HealthComponent.currentHealth` 0.0 _healthcomponent)
      (`self.Zazi Death`)))
  (bind _returnvalue_2 (`PrimitiveComponent.CreateDynamicMaterialInstance` (`self.Mesh`) 1 "/Game/Materials/Zazi/M_Zazi_Eyes.M_Zazi_Eyes" "None"))
  (`MaterialInstanceDynamic.SetVectorParameterValue` _returnvalue_2 "EyeLoc" (struct :`G` 0.33 :`A` 1.0))
  (`|PlayMontage` (`self.Mesh`) "/Game/Animations/Zazi/Movement/AM_Zazi_Hit.AM_Zazi_Hit"
    (:`OnNotifyBegin`
      (`self.DisableInput` null)
      (`KismetSystemLibrary.Delay` 2.0)
      (set `self.IsHit` false)
      (`self.EnableInput` null)
      (bind _returnvalue_3 (`PrimitiveComponent.CreateDynamicMaterialInstance` (`self.Mesh`) 1 "/Game/Materials/Zazi/M_Zazi_Eyes.M_Zazi_Eyes" "None"))
      (`MaterialInstanceDynamic.SetVectorParameterValue` _returnvalue_3 "EyeLoc" (struct :`A` 1.0)))))

(event `self.PlayBatteryTransition`
  ;[1 1 1] Battery Camera
  (`self.DisableInput` (`GameplayStatics.GetPlayerController` 0))
  (bind _returnvalue (`PrimitiveComponent.CreateDynamicMaterialInstance` (`self.Mesh`) 1 "/Game/Materials/Zazi/M_Zazi_Eyes.M_Zazi_Eyes" "None"))
  (`MaterialInstanceDynamic.SetVectorParameterValue` _returnvalue "EyeLoc" (struct :`R` 0.33 :`A` 1.0))
  (`|PlayMontage` (`self.Mesh`) "/Game/Animations/Zazi/Movement/AM_Zazi_BatteryCollect.AM_Zazi_BatteryCollect"
    (:`then`
      (bind (_direction _cameralerp) (`Timeline|Start Camera Transition` :!via `PlayFromStart`)
        (:`Update`
          (`SceneComponent.K2_SetWorldTransform` (`self.FollowCamera`) (`KismetMathLibrary.TLerp` (`SceneComponent.K2_GetComponentToWorld` (`self.FollowCamera`)) (`SceneComponent.K2_GetComponentToWorld` (`self.CameraTransition`)) _cameralerp) false false))
        (:`Finished`
          (`ActorComponent.SetActive` (`self.FollowCamera`) false false)
          (`ActorComponent.SetActive` (`self.CameraTransition`) true false))))
    (:`OnNotifyBegin`
      (`self.StopAnimMontage` "/Game/Animations/Zazi/Movement/AM_Zazi_BatteryCollect.AM_Zazi_BatteryCollect")
      (bind (_direction_2 _cameralerp_2) (`Timeline|Start Origin Camera Transition` :!via `ReverseFromEnd`)
        (:`Update`
          (`SceneComponent.K2_SetWorldTransform` (`self.FollowCamera`) (`KismetMathLibrary.TLerp` (`SceneComponent.K2_GetComponentToWorld` (`self.CameraOrigin`)) (`SceneComponent.K2_GetComponentToWorld` (`self.FollowCamera`)) _cameralerp_2) false false)
          (`ActorComponent.SetActive` (`self.FollowCamera`) true false)
          (`ActorComponent.SetActive` (`self.CameraTransition`) false false))
        (:`Finished`
          (bind _returnvalue_2 (`PrimitiveComponent.CreateDynamicMaterialInstance` (`self.Mesh`) 1 "/Game/Materials/Zazi/M_Zazi_Eyes.M_Zazi_Eyes" "None"))
          (`MaterialInstanceDynamic.SetVectorParameterValue` _returnvalue_2 "EyeLoc" (struct :`A` 1.0))
          (`self.EnableInput` (`GameplayStatics.GetPlayerController` 0)))))))

(fn `UserConstructionScript`)