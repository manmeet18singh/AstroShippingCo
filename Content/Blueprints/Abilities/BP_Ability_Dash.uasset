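; Dash ability actor that registers itself as the player character's current ability on BeginPlay and hides the crosshairs.
; On press, if cooled down and unlocked, it starts a hover effect, montage and sound, while a timeline drives velocity along the character's forward vector.
; Timeline updates reset the cooldown, which refills through a Delay loop and toggles the cooldown widget.
; Montage completion clears the dash lock; releasing the input stops the effect.
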(event `self.ReceiveBeginPlay`
  (bind _crosshairs (`/Game/Blueprints/PlayerController/BP_PlayerController.Crosshairs` (`self.Character`)))
  ;[1 1 1] Initialize Zazi's current ability
  (bind _asbp_player_controller (cast `/Game/Blueprints/PlayerController/BP_PlayerController` (`GameplayStatics.GetPlayerCharacter` 0)))
  (set `/Game/Blueprints/PlayerController/BP_PlayerController.Current Ability` self _asbp_player_controller)
  (bind _output_get (set `self.Character` _asbp_player_controller))
  (`SceneComponent.ToggleVisibility` (`/Game/Blueprints/PlayerController/BP_PlayerController.AbilityCooldownWidget` _output_get) false)
  (if (`SceneComponent.IsVisible` _crosshairs)
    (`SceneComponent.ToggleVisibility` _crosshairs false)))

(event `self.AbilityPressed`
  (bind _abilitycooldownwidget (`/Game/Blueprints/PlayerController/BP_PlayerController.AbilityCooldownWidget` (`self.Character`)))
  ;[1 1 1] Dash on Click
  (if (>= (`self.Cooldown Time`) 1.0)
    (if (not (`SceneComponent.IsVisible` _abilitycooldownwidget))
      (`SceneComponent.ToggleVisibility` _abilitycooldownwidget false))
    (if (not (`self.Dash Lock`))
      (set `self.Dash Lock` true)
      (`ActorComponent.Activate` (`self.Hover Effect 1`) false)
      (`|PlayMontage` (`Character.Mesh` (`self.Character`)) (`self.Mon_A`)
        (:`then`
          (`GameplayStatics.PlaySound2D` "/Game/Audio/SFX/PowerUps/Dash/DashCue.DashCue" 1.0 1.0 0.0 null null)
          (bind (_direction _distance_multiplier) (`Timeline|Movement` :!via `PlayFromStart`)
            (:`Update`
              (set `MovementComponent.Velocity` (* (`self.GetActorForwardVector` (`self.Character`)) (* _distance_multiplier (`self.MoveDistance`))) (`Character.CharacterMovement` (`self.Character`)))
              (set `self.Cooldown Time` 0.0)
              (if (< (`self.Cooldown Time`) 1.0) :!label _label
                (set `self.Cooldown Time` (+ (`self.Cooldown Time`) 0.2))
                (`KismetSystemLibrary.Delay` 0.3)
                (goto _label)
                (else
                  (`SceneComponent.ToggleVisibility` (`/Game/Blueprints/PlayerController/BP_PlayerController.AbilityCooldownWidget` (`self.Character`)) false))))))
        (:`OnCompleted`
          (set `self.Dash Lock` false))))))

(event `self.AbilityReleased`
  ;[1 1 1] Stop Dash Particle Effect
  (`ActorComponent.Deactivate` (`self.Hover Effect 1`)))

(fn `UserConstructionScript`)