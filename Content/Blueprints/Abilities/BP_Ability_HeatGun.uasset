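; Heat gun ability actor that registers itself as the player character's current ability on BeginPlay and creates a WBP_Jetpack widget as its HUD.
; When pressed off cooldown, it shows the HUD and plays a montage whose notify spawns a scaled-up BP_FireBall at the character's projectile reference.
; A Delay loop then refills the cooldown in steps and removes the HUD when full.
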(event `self.ReceiveBeginPlay`
  ;[1 1 1] Initialize Zazi's current ability
  (bind _asbp_player_controller (cast `/Game/Blueprints/PlayerController/BP_PlayerController` (`GameplayStatics.GetPlayerCharacter` 0)))
  (set `/Game/Blueprints/PlayerController/BP_PlayerController.Current Ability` self _asbp_player_controller)
  (set `self.Character` _asbp_player_controller)
  (bind _returnvalue (`|CreateWidget` "/Game/HUD/Overlay/WBP_Jetpack.WBP_Jetpack_C"))
  (set `self.HUD` _returnvalue))

(event `self.AbilityPressed`
  (bind _projectile_ref (`/Game/Blueprints/PlayerController/BP_PlayerController.Projectile Ref` (`self.Character`)))
  ;[1 1 1] Fire Gun (Replace With C++)
  (if (>= (`self.Cooldown Time`) 1.0)
    (if (not (`Widget.IsInViewport` (`self.HUD`)))
      (`UserWidget.AddToViewport` (`self.HUD`) 0))
    (`|PlayMontage` (`Character.Mesh` (`GameplayStatics.GetPlayerCharacter` 0)) (`self.Mon_A`) 0.8
      (:`OnNotifyBegin`
        (`|SpawnActorFromClass` "/Game/Blueprints/Projectiles/BP_FireBall.BP_FireBall_C" (`KismetMathLibrary.MakeTransform` (`SceneComponent.K2_GetComponentLocation` _projectile_ref) (`KismetMathLibrary.MakeRotFromZ` (`SceneComponent.GetForwardVector` _projectile_ref)) (2.0 2.0 2.0)) "Undefined" "OverrideRootScale" null null)
        (set `self.Cooldown Time` 0.0)
        (if (< (`self.Cooldown Time`) 1.0) :!label _label
          (set `self.Cooldown Time` (+ (`self.Cooldown Time`) 0.1))
          (`KismetSystemLibrary.Delay` 0.2)
          (goto _label)
          (else
            (`Widget.RemoveFromParent` (`self.HUD`))))))))

(fn `UserConstructionScript`)