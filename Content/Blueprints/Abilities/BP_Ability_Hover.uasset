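; Jetpack hover ability that registers as the player's current ability and lets them fly on limited fuel.
; Pressing sets Flying movement, shows the jetpack HUD, starts sound and effects, and runs a looping fuel-drain timer.
; Release restores Walking, stops the feedback, and starts a regen timer, as does running out of fuel.
; Regen refuels only while grounded, removing the HUD once full.
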(event `self.ReceiveBeginPlay`
  ;[1 1 1] Initialize Zazi's current ability
  (bind _asbp_player_controller (cast `/Game/Blueprints/PlayerController/BP_PlayerController` (`GameplayStatics.GetPlayerCharacter` 0)))
  (set `/Game/Blueprints/PlayerController/BP_PlayerController.Current Ability` self _asbp_player_controller)
  (set `self.Character` _asbp_player_controller)
  (bind _returnvalue (`|CreateWidget` "/Game/HUD/Overlay/WBP_Jetpack.WBP_Jetpack_C"))
  (set `self.HUD` _returnvalue))

(event `self.AbilityPressed`
  (bind _hud (`self.HUD`))
  ;[1 1 1] Pressed
  (if (not (`Widget.IsInViewport` _hud))
    (`UserWidget.AddToViewport` _hud 0))
  (`CharacterMovementComponent.SetMovementMode` (`Character.CharacterMovement` (`self.Character`)) "MOVE_Flying" 0)
  (bind _returnvalue (`GameplayStatics.SpawnSound2D` "/Game/Audio/SFX/PowerUps/JetPack/JetpackCue.JetpackCue" 1.0 1.0 0.0 null))
  (set `self.SFX` _returnvalue)
  (`ActorComponent.Activate` (`self.Hover Effect 1`) false)
  (`ActorComponent.Activate` (`self.Hover Effect 2`) false)
  (bind _returnvalue_2 (`KismetSystemLibrary.K2_SetTimerDelegate` (delegate `Deplete Fuel`) 0.05 true)) ; Fuel Deplete Timer
  (`KismetSystemLibrary.K2_ClearAndInvalidateTimerHandle` (stale `self.AbilityReleased` _returnvalue)) ; Clear Refueling Timer
  (`KismetSystemLibrary.K2_ClearAndInvalidateTimerHandle` (stale `Deplete Fuel` _returnvalue)) ; Clear refueling start timer
)

(event `Deplete Fuel`
  ;[1 1 1] Pressed
  (if (>= (`self.Current Fuel`) 5.0)
    (bind _output_get (set `self.Current Fuel` (- (`self.Current Fuel`) (`self.Depletion Rate`))))
    (if (<= _output_get 0.0)
      (`CharacterMovementComponent.SetMovementMode` (`Character.CharacterMovement` (`self.Character`)) "MOVE_Walking" 0)
      (`ActorComponent.Deactivate` (`self.Hover Effect 1`))
      (`ActorComponent.Deactivate` (`self.Hover Effect 2`))
      (`AudioComponent.Stop` (`self.SFX`))
      (`KismetSystemLibrary.K2_ClearAndInvalidateTimerHandle` (stale `self.AbilityPressed` _returnvalue_2)) ; Clear deplete timer after all the fuel's depleated
      (bind _returnvalue (`KismetSystemLibrary.K2_SetTimerDelegate` (delegate `Regen Fuel`) 0.05 true)) ; Timer for when to start refueling
    )))

(event `self.AbilityReleased`
  ;[1 1 1] Released
  (`CharacterMovementComponent.SetMovementMode` (`Character.CharacterMovement` (`self.Character`)) "MOVE_Walking" 0)
  (`ActorComponent.Deactivate` (`self.Hover Effect 1`))
  (`ActorComponent.Deactivate` (`self.Hover Effect 2`))
  (if (`AudioComponent.IsPlaying` (`self.SFX`))
    (`AudioComponent.Stop` (`self.SFX`)))
  (bind _returnvalue (`KismetSystemLibrary.K2_SetTimerDelegate` (delegate `Regen Fuel`) 0.05 true))
  (`KismetSystemLibrary.K2_ClearAndInvalidateTimerHandle` (stale `self.AbilityPressed` _returnvalue_2)) ; Clear Fuel Deplete Timer
)

(event `Regen Fuel`
  (bind _hud (`self.HUD`))
  (bind _charactermovement (`Character.CharacterMovement` (`self.Character`)))
  ;[1 1 1] Released
  (if (and (not (`NavMovementComponent.IsFlying` _charactermovement)) (not (`NavMovementComponent.IsFalling` _charactermovement)))
    (if (>= (`self.Current Fuel`) (`self.Max Fuel`))
      (`KismetSystemLibrary.K2_ClearAndInvalidateTimerHandle` (stale `self.AbilityReleased` _returnvalue)) ; When finished Refueling Stop Refueling Timer
      (`KismetSystemLibrary.K2_ClearAndInvalidateTimerHandle` (stale `Deplete Fuel` _returnvalue)) ; Clear fueling timer
      (if (`Widget.IsInViewport` _hud)
        (`Widget.RemoveFromParent` _hud))
      (else
        (set `self.Current Fuel` (+ (`self.Current Fuel`) (`self.Regen Rate`)))))))

(fn `Drop`)

(fn `UserConstructionScript`)