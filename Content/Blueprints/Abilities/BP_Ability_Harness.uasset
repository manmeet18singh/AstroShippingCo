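; Harness ability that lets the player push the character's current pushable object while the ability button is held.
; Begin Play registers it as the current ability and hides the crosshair and cooldown widgets.
; Pressing attaches the character to the object, constrains movement to the facing plane and starts push audio and Tick, which sweeps the object forward at its push speed.
; Release detaches, restores movement and stops audio and Tick.
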(event `self.ReceiveBeginPlay`
  (bind _character (`self.Character`))
  (bind _crosshairs (`/Game/Blueprints/PlayerController/BP_PlayerController.Crosshairs` _character))
  ;[1 1 1] Begin Play
  (bind _asbp_player_controller (cast `/Game/Blueprints/PlayerController/BP_PlayerController` (`GameplayStatics.GetPlayerCharacter` 0)))
  (set `/Game/Blueprints/PlayerController/BP_PlayerController.Current Ability` self _asbp_player_controller)
  (set `self.Character` _asbp_player_controller)
  (`self.SetActorTickEnabled` false)
  (if (or (`SceneComponent.IsVisible` _crosshairs) (`SceneComponent.IsVisible` (`/Game/Blueprints/PlayerController/BP_PlayerController.AbilityCooldownWidget` _character)))
    (`SceneComponent.SetVisibility` _crosshairs false false)
    (`SceneComponent.SetVisibility` (`/Game/Blueprints/PlayerController/BP_PlayerController.AbilityCooldownWidget` _character) false false)))

(event `self.ReceiveTick`
  (params (DeltaSeconds :type "Float (single-precision)"))
  ;[1 1 1] Push Object Logic
  (bind _pushable (`self.Pushable`)
    (:`then`
      (`self.K2_AddActorWorldOffset` _pushable (* (`self.GetActorForwardVector` (`self.Character`)) (* DeltaSeconds (`/Game/Blueprints/Pickups/BP_Pickup_Pushable.Push Speed` _pushable))) true false))
    (:`else`)))

(event `self.AbilityPressed`
  ;[1 1 1] Start Pushing Object
  (bind _current_push (`/Game/Blueprints/PlayerController/BP_PlayerController.Current Push` (`self.Character`))
    (:`then`
      (bind _output_get (set `self.Pushable` _current_push))
      (`self.Begin Push` _output_get) ; Attach Box to Zazi
    )
    (:`else`)))

(event `self.AbilityReleased`
  ;[1 1 1] Stop Push
  (bind _current_push (`/Game/Blueprints/PlayerController/BP_PlayerController.Current Push` (`self.Character`))
    (:`then`
      (`ActorComponent.Activate` (`/Game/Blueprints/Pickups/BP_Pickup_Pushable.StandParticle1` _current_push) false)
      (`ActorComponent.Activate` (`/Game/Blueprints/Pickups/BP_Pickup_Pushable.StandParticle2` _current_push) false)
      (`ActorComponent.Activate` (`/Game/Blueprints/Pickups/BP_Pickup_Pushable.StandParticle3` _current_push) false)
      (`ActorComponent.Activate` (`/Game/Blueprints/Pickups/BP_Pickup_Pushable.StandParticle4` _current_push) false)
      (`self.End Push`) ; Detach Box from Zazi
    )
    (:`else`)))

(fn `Begin Push`
  (params (Pushable :type "/Game/Blueprints/Pickups/BP_Pickup_Pushable Object Reference"))
  (bind _character (`self.Character`))
  (bind _character_2 (`self.Character`))
  (bind _charactermovement (`Character.CharacterMovement` _character_2))
  (`self.K2_AttachToActor` (`self.Character`) Pushable "None" "KeepWorld" "KeepWorld" "KeepWorld" true)
  (`MovementComponent.SetPlaneConstraintEnabled` _charactermovement true)
  (`MovementComponent.SetPlaneConstraintNormal` _charactermovement (`self.GetActorRightVector` _character_2))
  (set `CharacterMovementComponent.bOrientRotationToMovement` false _charactermovement)
  (set `AstroShippingCoCharacter.isPushing` true _character)
  (bind _returnvalue (`GameplayStatics.SpawnSoundAtLocation` "/Game/Audio/SFX/PowerUps/Harness/Push_Cue.Push_Cue" (`self.K2_GetActorLocation` _character) (struct) 1.0 1.0 0.0 null null))
  (bind _output_get (set `self.SFX` _returnvalue))
  (`AudioComponent.Play` _output_get 0.0)
  (`self.SetActorTickEnabled` true))

(fn `End Push`
  (bind _charactermovement (`Character.CharacterMovement` (`self.Character`)))
  (`self.Pushable`
    (:`then`
      (set `self.Pushable` null)
      (`self.K2_DetachFromActor` (`self.Character`) "KeepWorld" "KeepWorld" "KeepWorld")
      (`MovementComponent.SetPlaneConstraintEnabled` _charactermovement false)
      (set `CharacterMovementComponent.bOrientRotationToMovement` true _charactermovement)
      (set `AstroShippingCoCharacter.isPushing` false (`self.Character`))
      (`AudioComponent.Stop` (`self.SFX`))
      (`self.SetActorTickEnabled` false))
    (:`else`)))

(fn `UserConstructionScript`)