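; Enemy character that roams the level, chases pawns it sees and can be killed through its head hitbox.
; Random roaming loops through AIMoveTo, while Pawn Sensing redirects it to the seen pawn and resumes roaming after a retriggerable delay.
; HeadBox overlap with BP_PlayerController or BP_FireBall stops and destroys it; Damage_Box overlap sends damage to the other actor.
; It tracks speed, attacking and death states; TakeDamage is an empty stub with disconnected health logic.
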(event `self.ReceiveBeginPlay`
  ;[1 1 1] Setting Player and Health Widget References
  (`self.Random Roam`)
  (castclass `/Game/Blueprints/PlayerController/BP_PlayerController` (`GameplayStatics.GetObjectClass` (`GameplayStatics.GetPlayerController` 0)))
  (set `self.BP Player Controller` "/Game/Blueprints/PlayerController/BP_PlayerController.BP_PlayerController"))

(event `Random Roam`
  ;[1 1 1] Setting Player and Health Widget References
  (`|AIMoveTo` self (`NavigationSystemV1.K2_GetRandomReachablePointInRadius` (`self.K2_GetActorLocation`) 1500.0 null null) null
    (:`OnSuccess`
      (`self.Random Roam`))))

(event `self.PawnSensing.OnSeePawn`
  (params (Pawn :type "Pawn Object Reference"))
  ;[1 1 1] Pawn Sensing to Follow Player
  (`|ExecutionSequence`
    (:`then_0`
      (`|AIMoveTo` self (0.0 0.0 0.0) Pawn))
    (:`then_1`
      (`KismetSystemLibrary.RetriggerableDelay` 1.0)
      (`self.Random Roam`))))

(event `self.HeadBox.OnComponentBeginOverlap`
  (params (OverlappedComponent :type "PrimitiveComponent Object Reference") (OtherActor :type "Actor Object Reference") (OtherComp :type "PrimitiveComponent Object Reference") (OtherBodyIndex :type Integer) (bFromSweep :type Boolean) (SweepResult :type "HitResult Structure (by ref)"))
  (bind _charactermovement (`self.CharacterMovement`))
  ;[1 1 1] Stomp Logic
  (`|ExecutionSequence`
    (:`then_0`
      (cast `/Game/Blueprints/PlayerController/BP_PlayerController` OtherActor))
    (:`then_1`
      (cast `/Game/Blueprints/Projectiles/BP_FireBall` OtherActor)))
  (`GameplayStatics.PlaySoundAtLocation` "/Game/Audio/SFX/Enemy_Hurt_Sound.Enemy_Hurt_Sound" (`self.K2_GetActorLocation`) (struct) 1.0 1.0 0.0 null null null)
  (`ActorComponent.K2_DestroyComponent` (`self.HeadBox`))
  (`ActorComponent.K2_DestroyComponent` (`self.Damage_Box`))
  (`MovementComponent.StopMovementImmediately` _charactermovement)
  (`CharacterMovementComponent.DisableMovement` _charactermovement)
  (set `self.IsDead` true)
  (`KismetSystemLibrary.Delay` 1.0)
  (`self.K2_DestroyActor`))

(event `self.Damage_Box.OnComponentBeginOverlap`
  (params (OverlappedComponent :type "PrimitiveComponent Object Reference") (OtherActor :type "Actor Object Reference") (OtherComp :type "PrimitiveComponent Object Reference") (OtherBodyIndex :type Integer) (bFromSweep :type Boolean) (SweepResult :type "HitResult Structure (by ref)"))
  ;[1 1 1] Damage to the Player
  (set `self.IsAttacking` true)
  (message `/Game/Blueprints/PlayerController/BPI_Damageable.Take Damage` OtherActor 25.0)
  (`KismetSystemLibrary.Delay` 10.0))

(event `self.ReceiveTick`
  (params (DeltaSeconds :type "Float (single-precision)"))
  ;[1 1 1] Calc Speed
  (set `self.Speed` (`KismetMathLibrary.VSize` (`self.GetVelocity`))))

(event `self.Damage_Box.OnComponentEndOverlap`
  (params (OverlappedComponent :type "PrimitiveComponent Object Reference") (OtherActor :type "Actor Object Reference") (OtherComp :type "PrimitiveComponent Object Reference") (OtherBodyIndex :type Integer))
  ;[1 1 1] Stop Attacking Bool
  (set `self.IsAttacking` false))

(event `/Game/Blueprints/PlayerController/BPI_Damageable.Take Damage`
  (params (Damage :type "Float (single-precision)"))
  ;[1 1 1] Take Damage from Projectile
)

(fn `UserConstructionScript`)