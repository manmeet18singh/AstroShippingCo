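; Enemy turret that shoots at pawns it sees and dies when hit by a BP_FireBall.
; Pawn Sensing yaws the mesh toward the seen pawn, then after a short delay spawns an actor at the BulletSpawner socket with a fire sound.
; A fireball overlapping the box collider plays an explosion, removes a collider, squashes the actor vertically, then destroys it after a brief delay.
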(event `self.PawnSensing.OnSeePawn`
  (params (Pawn :type "Pawn Object Reference"))
  (bind (_returnvalue_roll _returnvalue_pitch _returnvalue_yaw) (`KismetMathLibrary.BreakRotator` (`KismetMathLibrary.FindLookAtRotation` (`SceneComponent.K2_GetComponentLocation` (`self.Turret_Mesh`)) (`self.K2_GetActorLocation` Pawn))))
  ;[1 1 1] Pawn Sensing/Sphere Collision to Player Controller
  (`SceneComponent.K2_SetRelativeRotation` (`self.Turret_Mesh`) (`KismetMathLibrary.MakeRotator` 0.0 0.0 _returnvalue_yaw) false false)
  (`KismetSystemLibrary.Delay` 1.0)
  (`|SpawnActorFromClass` "/Game/Blueprints/Enemies/BP_Projectile.BP_Projectile_C" (`SceneComponent.GetSocketTransform` (`self.Bullet_Spawner`) "Bulllet" "RTS_World") "Undefined" "OverrideRootScale" null null)
  (`GameplayStatics.PlaySound2D` "/Game/Audio/SFX/Turret_Bass_Fire_SFX.Turret_Bass_Fire_SFX" 1.0 1.0 0.0 null null))

(event `self.Box_Colldier.OnComponentBeginOverlap`
  (params (OverlappedComponent :type "PrimitiveComponent Object Reference") (OtherActor :type "Actor Object Reference") (OtherComp :type "PrimitiveComponent Object Reference") (OtherBodyIndex :type Integer) (bFromSweep :type Boolean) (SweepResult :type "HitResult Structure (by ref)"))
  ;[1 1 1] Enemy SFX and Enemy Death Animation
  (cast `/Game/Blueprints/Projectiles/BP_FireBall` OtherActor)
  (`GameplayStatics.PlaySoundAtLocation` "/Game/Audio/SFX/ExplosionCompute_CRB01_71_1.ExplosionCompute_CRB01_71_1" (`self.K2_GetActorLocation`) (struct) 1.0 1.0 0.0 null null null)
  (`ActorComponent.K2_DestroyComponent` (`self.Box_Colldier`))
  (`SceneComponent.SetWorldScale3D` (`self.DefaultSceneRoot`) (1.0 1.0 0.5))
  (`KismetSystemLibrary.Delay` 0.5)
  (`self.K2_DestroyActor`))

(fn `UserConstructionScript`)