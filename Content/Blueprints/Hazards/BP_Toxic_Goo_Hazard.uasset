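; Toxic goo hazard that damages the player and shows a toxic status widget while they are inside it.
; Creates WBP_Status_Toxic at BeginPlay, then adds or removes it from the viewport as BP_PlayerController actors begin or end overlap with Damage_Box.
; Damage is a single TakeDamageMessage call on entry, with no repeat while overlapping.
; The Delay after exit leads to nothing.
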(event `self.ReceiveBeginPlay`
  (bind _returnvalue (`|CreateWidget` "/Game/HUD/WBP_Status_Toxic.WBP_Status_Toxic_C"))
  (set `self.Widget Ref` _returnvalue))

(event `self.Damage_Box.OnComponentBeginOverlap`
  (params (OverlappedComponent :type "PrimitiveComponent Object Reference") (OtherActor :type "Actor Object Reference") (OtherComp :type "PrimitiveComponent Object Reference") (OtherBodyIndex :type Integer) (bFromSweep :type Boolean) (SweepResult :type "HitResult Structure (by ref)"))
  (bind _asbp_player_controller (cast `/Game/Blueprints/PlayerController/BP_PlayerController` OtherActor))
  (message `/Game/Blueprints/PlayerController/BPI_Damageable.Take Damage` _asbp_player_controller 1.0)
  (`self.Damage Indicator` true))

(event `self.Damage_Box.OnComponentEndOverlap`
  (params (OverlappedComponent :type "PrimitiveComponent Object Reference") (OtherActor :type "Actor Object Reference") (OtherComp :type "PrimitiveComponent Object Reference") (OtherBodyIndex :type Integer))
  (cast `/Game/Blueprints/PlayerController/BP_PlayerController` OtherActor)
  (`self.Damage Indicator` false)
  (`KismetSystemLibrary.Delay` 0.2))

(fn `Damage Indicator`
  (params (`Add To Screen?` :type Boolean))
  (if `Add To Screen?`
    (`UserWidget.AddToViewport` (`self.Widget Ref`) 0)
    (else
      (`Widget.RemoveFromParent` (`self.Widget Ref`)))))

(fn `UserConstructionScript`)